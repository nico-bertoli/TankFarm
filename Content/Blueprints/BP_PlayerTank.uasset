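; Player tank Blueprint that tracks whether the tank is touching the ground.
; Overlap events on the GroundContactDetector component set and clear IsTouchingGround for any actor other than itself, without counting simultaneous overlaps.
; Both events print the other actor's name as debug output.
; An IsNotTankCollider helper checks for the TankCollider component tag but returns no value and is not called here.
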(event OnComponentBeginOverlap(GroundContactDetector)
  (params (OverlappedComponent :type Primitive%20Component%20Object%20Reference) (OtherActor :type Actor%20Object%20Reference) (OtherComp :type Primitive%20Component%20Object%20Reference) (OtherBodyIndex :type Integer) (bFromSweep :type Boolean) (SweepResult :type Hit%20Result%20Structure%20%28by%20ref%29))
  (if (not (== OtherActor self))
    (Variables|Default|SetIsTouchingGround true)
    (Development|PrintString (Utilities|GetDisplayName OtherActor) true true "(R=0.000000,G=0.660000,B=1.000000,A=1.000000)" 1e+01)))

(event OnComponentEndOverlap(GroundContactDetector)
  (params (OverlappedComponent :type Primitive%20Component%20Object%20Reference) (OtherActor :type Actor%20Object%20Reference) (OtherComp :type Primitive%20Component%20Object%20Reference) (OtherBodyIndex :type Integer))
  (if (not (== OtherActor self))
    (Variables|Default|SetIsTouchingGround false)
    (Development|PrintString (Utilities|GetDisplayName OtherActor) true true "(R=1.000000,G=0.000000,B=0.012991,A=1.000000)" 1e+01)))

(event EventBeginPlay)

(event Collision|EventActorBeginOverlap
  (params (OtherActor :type Actor%20Object%20Reference)))

(event EventTick
  (params (DeltaSeconds :type Float%20%28single-precision%29)))

(fn ConstructionScript)

(fn IsNotTankCollider
  (params (self2 :type Actor%20Component%20Object%20Reference))
  (if (not (Utilities|Array|ContainsItem (Variables|/Script/Engine.ActorComponent|GetComponentTags self2) "TankCollider"))
    (return)))